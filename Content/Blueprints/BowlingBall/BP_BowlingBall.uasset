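; Grabbable VR bowling ball that carries a camera aimed at the player holding it.
; Its grab component caches the grabbing VRPawn's HMD, sets the grabbed state and fires the GotGrabbed dispatcher.
; While held, Tick turns the camera toward that HMD with a look-at rotation; otherwise it holds a zero world rotation.
; Dropping clears the grabbed state and resets the camera's relative position above the ball.
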(event OnDropped(GrabComponent)
  (Variables|Default|SetIsBallGrabbed false)
  (Transformation|SetRelativeLocation (Variables|Default|GetCamera) "0.000000,0.000000,50.000000" false false))

(event OnGrabbed(GrabComponent)
  (params (Grabbing%20Controller :type Motion%20Controller%20Component%20Object%20Reference))
  (bind _asvrpawn (Utilities|Casting|CastToVRPawn (Components|GetOwner Grabbing%20Controller)))
  (Variables|Default|SetGrabbed%20Owner%20HMD (Variables|/Game/VRTemplate/Blueprints/VRPawn.VRPawn_C|GetHMD _asvrpawn))
  (Variables|Default|SetIsBallGrabbed true)
  (Default|CallGotGrabbed self))

(event EventTick
  (params (DeltaSeconds :type Float%20%28single-precision%29))
  (bind _camera (Variables|Default|GetCamera))
  (if (Variables|Default|GetIsBallGrabbed)
    (bind _desiredview (Class|CameraComponent|GetCameraView _camera 0.0))
    (Transformation|SetWorldRotation _camera (Math|Rotator|FindLookatRotation (.Location (Utilities|Struct|BreakMinimalViewInfo _desiredview)) (Transformation|GetWorldLocation (Variables|Default|GetGrabbed%20Owner%20HMD))) false false)
    (else
      (Transformation|SetWorldRotation (Variables|Default|GetCamera) "0, 0, 0" false false))))

(fn ConstructionScript)