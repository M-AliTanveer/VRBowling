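; VR grippable bowling ball that tracks who holds it, steers its own camera and boosts the throw on release.
; Grip and drop events set the holder and grip state, then fire dispatchers announcing the change.
; Each tick the camera sits at its local origin facing the holder's head while gripped, otherwise offset upward with zero world rotation.
; Release scales horizontal velocity up and zeroes vertical velocity.
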(event Custom|Set%20Camera%20Movement%20for%20All
  (bind _camera (Variables|Default|GetCamera))
  (bind _camera_2 (Variables|Default|GetCamera))
  (if (Variables|Default|Getis%20Gripped)
    (bind _desiredview (Class|CameraComponent|GetCameraView (Variables|Default|GetCamera) 0.0))
    (Transformation|SetWorldRotation _camera (Math|Rotator|FindLookatRotation (.Location (Utilities|Struct|BreakMinimalViewInfo _desiredview)) (Class|VRBaseCharacter|GetVRHeadLocation (Variables|Default|GetHolding%20Character))) false false)
    (Transformation|SetRelativeLocation _camera "0, 0, 0" false false)
    (else
      (Transformation|SetWorldRotation _camera_2 "0, 0, 0" false true)
      (Transformation|SetRelativeLocation _camera_2 "0.000000,0.000000,50.000000" false false))))

(event EventBeginPlay
  (EventDispatchers|BindEventtoOnGripped (delegate BallGripped))
  (EventDispatchers|BindEventtoOnDropped (delegate BallReleased)))

(event EventTick
  (params (DeltaSeconds :type Float%20%28single-precision%29))
  (CallFunction|SetCameraMovementforAll))

(fn ConstructionScript)

(event Custom|OnGripped_Event
  (params (GrippingController :type Grip%20Motion%20Controller%20Component%20Object%20Reference) (GripInformation :type BP%20Actor%20Grip%20Information%20Structure%20%28by%20ref%29))
  (bind _asbp_vrcharacter (Utilities|Casting|CastToBP_VRCharacter (Components|GetOwner GrippingController)))
  (Variables|Default|SetHolding%20Character _asbp_vrcharacter)
  (Variables|Default|Setis%20Gripped true)
  (Default|CallBallGrippedbyPlayer self))

(event Custom|OnDropped_Event
  (params (GrippingController :type Grip%20Motion%20Controller%20Component%20Object%20Reference) (GripInformation :type BP%20Actor%20Grip%20Information%20Structure%20%28by%20ref%29) (bWasSocketed :type Boolean))
  (bind _returnvalue (Transformation|GetVelocity))
  (Class|PrimitiveComponent|SetAllPhysicsLinearVelocity (Variables|Default|GetStaticMeshComponent) (* (Math|Vector|MakeVector (.x _returnvalue) (.y _returnvalue) 0.0) 1.5) false)
  (Variables|Default|Setis%20Gripped false)
  (Default|CallBallReleasedbyPlayer))