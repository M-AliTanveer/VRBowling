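; Game mode for a VR prototype level that hosts an Epic Online Services session on a dedicated server.
; On server BeginPlay it initializes EIK, then after a delay creates a two-slot session and records whether that succeeded.
; Login and logout maintain a list of VR player controllers, and each login requests an EOS voice room token with placeholder player details, printing the result.
; Two-player match start logic exists but is disconnected.
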(event Custom|CustomEvent
  (params (bWasSuccess :type Boolean) (RoomData :type String))
  (Development|PrintString (Utilities|String|ToString(Boolean) bWasSuccess))
  (Development|PrintString RoomData true true "(R=1.000000,G=0.126976,B=0.000000,A=1.000000)" 1e+01))

(event EventBeginPlay
  ;[1 1 1] Start Session at start of server
  (if (Networking|IsDedicatedServer)
    (bind _asgs_proto_level (Utilities|Casting|CastToGS_ProtoLevel (Game|GetGameState)))
    (Variables|Default|SetGame%20State _asgs_proto_level)
    (Class|EIKSubsystem|InitializeEIK (Subsystems|GetEIKSubsystem))
    (Utilities|FlowControl|Delay 5.0)
    (Class|EIKSubsystem|CreateEOSSession (Subsystems|GetEIKSubsystem) (delegate NewSessionCreated_2) (Utilities|Map|MakeMap "IsServer" "true") "Default_Session" true false 2 "RE_NoSelection")))

(event EventPostLogin
  (params (NewPlayer :type Player%20Controller%20Object%20Reference))
  ;[1 1 1] Maintain list of player controller
  (bind _asvr_player_controller (Utilities|Casting|CastToVR_Player_Controller NewPlayer))
  (Utilities|Array|Add (Variables|Server|GetConnectedPlayers) _asvr_player_controller)
  (Class|EVIKFunctions|EOSRoomToken _asvr_player_controller "Play" "test" "10.0.0.1" (delegate Custom|CustomEvent)))

(event EventOnLogout
  (params (ExitingController :type Controller%20Object%20Reference))
  ;[1 1 1] Maintain list of player controller
  (bind _asvr_player_controller (Utilities|Casting|CastToVR_Player_Controller ExitingController))
  (Utilities|Array|RemoveItem (Variables|Server|GetConnectedPlayers) _asvr_player_controller))

(fn ConstructionScript)

(event Custom|Session%20Created
  (params (bWasSuccess :type Boolean) (SessionName :type Name%20%28by%20ref%29))
  (bind _output_get (Variables|Server|SetisServerRunning bWasSuccess))
  (Development|PrintString (Utilities|String|ToString(Boolean) _output_get)))