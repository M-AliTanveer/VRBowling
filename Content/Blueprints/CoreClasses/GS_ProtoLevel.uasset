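; Game state for a two-player, turn-based bowling level, tracking match status, round, connected players and whose turn it is.
; StartMatch stores the controllers, and ChangeTurn swaps pawn input between the two players, optionally advancing the round.
; When a ball is grabbed, the waiting player's camera blends to that ball, then returns to their own pawn on alley reset.
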(event Custom|Alley%20Reset
  (bind _current_player_index (Variables|Default|GetCurrent%20Player%20Index))
  (bind _connected_players (Variables|Default|GetConnected%20Players))
  (bind _returnvalue (- 1 _current_player_index))
  (bind _output (Utilities|Array|Get(acopy) _connected_players _returnvalue))
  ;[1 1 1] Camera Switching for Opponent
  (Utilities|FlowControl|Delay 0.01)
  (Game|Player|SetViewTargetwithBlend _output (Pawn|GetControlledPawn _output) 0.0 "VTBlend_EaseInOut" 0.0 false))

(event Custom|Change%20Turn
  (params (Round%20Changed :type Boolean))
  ;[1 1 1] Change Turn for Players
  (Input|DisableInput (Pawn|GetControlledPawn (Utilities|Array|Get(acopy) (Variables|Default|GetConnected%20Players) (Variables|Default|GetCurrent%20Player%20Index))) (Utilities|Array|Get(acopy) (Variables|Default|GetConnected%20Players) (Variables|Default|GetCurrent%20Player%20Index)))
  (Variables|Default|SetCurrent%20Player%20Index (- 1 (Variables|Default|GetCurrent%20Player%20Index)))
  (Input|EnableInput (Pawn|GetControlledPawn (Utilities|Array|Get(acopy) (Variables|Default|GetConnected%20Players) (Variables|Default|GetCurrent%20Player%20Index))) (Utilities|Array|Get(acopy) (Variables|Default|GetConnected%20Players) (Variables|Default|GetCurrent%20Player%20Index)))
  (Variables|Default|SetCurrent%20Turn%20Player (Utilities|Array|Get(acopy) (Variables|Default|GetConnected%20Players) (Variables|Default|GetCurrent%20Player%20Index)))
  (if Round%20Changed
    (Math|Integer|IncrementInt (Variables|Default|GetCurrent%20Round))))

(event Custom|Ball%20Grabbed%20by%20Player
  (params (Bowling%20Ball :type BP%20Bowling%20Ball%20Grip%20Object%20Reference))
  ;[1 1 1] Camera Switching for Opponent
  (Utilities|FlowControl|Delay 0.01)
  (Game|Player|SetViewTargetwithBlend (Utilities|Array|Get(acopy) (Variables|Default|GetConnected%20Players) (- 1 (Variables|Default|GetCurrent%20Player%20Index))) Bowling%20Ball 0.0 "VTBlend_EaseInOut" 0.0 false))

(event Custom|Start%20Match
  (params (Controllers%20in%20Play :type Array%20of%20VR%20Player%20Controller%20Object%20References) (Current%20Turn%20Player :type VR%20Player%20Controller%20Object%20Reference))
  ;[1 1 1] Set up match start attributes
  (Variables|Default|SetMatch%20in%20Play true)
  (Variables|Default|SetCurrent%20Round 0)
  (Variables|Default|SetConnected%20Players Controllers%20in%20Play)
  (Variables|Default|SetCurrent%20Turn%20Player Current%20Turn%20Player))

(event EventBeginPlay
  ;[1 1 1] Begin Play
  (bind _asgm_proto_level (Utilities|Casting|CastToGM_ProtoLevel (Game|GetGameMode)))
  (Variables|Default|SetGame%20Mode _asgm_proto_level))

(fn ConstructionScript)