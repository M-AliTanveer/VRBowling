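; Client game instance that handles Epic Online Services login, session joining and voice chat for a VR player.
; Init, skipped on dedicated servers, fetches the public IP, initializes EIK, spawns a 3D login widget near the VR character, then opens a hardcoded localhost server after delays.
; Device ID or Account Portal login starts a callback chain: join the first found session, connect voice, join the "BowlingGame" room using an IP-based token, then register the player.
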(event Custom|Join%20Session
  (params (bWasSuccess :type Boolean))
  (bind _returnvalue (Game|GetPlayerController 0))
  ;[1 1 1] Joining EOS Session
  (bind _output_get (Variables|Default|SetisConnectedToSession bWasSuccess))
  (if _output_get
    (Development|PrintString "Session Joined Success" true true "(R=1.000000,G=0.000000,B=0.028161,A=1.000000)" 5e+01)
    ;[1 1 1] Join EOS Voice Room
    (Class|EVIKFunctions|InitializeEOSVoiceChat _returnvalue)
    (Class|EVIKFunctions|ConnectVoiceChat _returnvalue (delegate Custom|EOS%20Voice%20Chat%20Connect))))

(event Custom|Join%20EOS%20voice%20Room
  (params (bWasSuccess :type Boolean) (Result :type EEVIKResultCodes%20Enum :default "Success"))
  ;[1 1 1] Join EOS Voice Room
  (bind _output_get (Variables|Default|SetisConnectedToVoiceChat bWasSuccess))
  (if _output_get
    (Development|PrintString "Voice Chat connected" true true "(R=1.000000,G=0.000000,B=0.135502,A=1.000000)" 5e+01)
    (Class|EIKSubsystem|RegisterPlayer (Subsystems|GetEIKSubsystem) "Default_Session" false)))

(event Custom|User%20Login
  (params (bWasSuccess :type Boolean) (Error :type String))
  ;[1 1 1] Logging In Using Device ID
  (if bWasSuccess
    (Development|PrintString "Login success" true true "(R=1.000000,G=0.000000,B=0.037282,A=1.000000)" 5e+01)
    (CallFunction|JoinEOSSession)))

(event Custom|Login%20Using%20Device%20ID
  (params (Username :type String))
  ;[1 1 1] Logging In Using Device ID
  (bind _output_get (Variables|Default|SetDeviceID%20username Username))
  (Class|EIKSubsystem|LoginwithDeviceID (Subsystems|GetEIKSubsystem) 0 _output_get "" (delegate Custom|User%20Login)))

(event Custom|Login%20using%20Account%20Portal
  ;[1 1 1] Logging In Using Account Portal
  (Class|EIKSubsystem|LoginwithAccountPortal (Subsystems|GetEIKSubsystem) 0 (delegate Custom|User%20Login)))

(event Custom|IP%20Received
  (params (IP :type String))
  ;[1 1 1] Get IP Address
  (Variables|Default|SetIP%20Address IP))

(event Custom|EOS%20Voice%20Chat%20Connect
  (params (bWasSuccess :type Boolean) (Result :type EEVIKResultCodes%20Enum :default "Success"))
  ;[1 1 1] Join EOS Voice Room
  (if bWasSuccess
    (Development|PrintString (Utilities|String|Append "Player Nickname: " (Variables|Default|GetDeviceID%20username)) true true "(R=1.000000,G=0.090672,B=0.000000,A=1.000000)" 5e+01)
    (Class|EVIKFunctions|LoginEOSVoiceChat (Game|GetPlayerController 0) (Variables|Default|GetDeviceID%20username) (delegate Custom|Login%20to%20EOS))))

(event Custom|Login%20to%20EOS
  (params (bWasSuccess :type Boolean) (Result :type EEVIKResultCodes%20Enum :default "Success"))
  (bind _returnvalue (Game|GetPlayerController 0))
  ;[1 1 1] Join EOS Voice Room
  (if bWasSuccess
    (Class|EVIKFunctions|EOSRoomToken _returnvalue "BowlingGame" (Class|EVIKFunctions|LoggedinUser _returnvalue) (Variables|Default|GetIP%20Address) (delegate Custom|Get%20voice%20room%20token))))

(event Custom|Join%20EOS%20Session
  ;[1 1 1] Joining EOS Session
  (Class|EIKSubsystem|FindEOSSession (Subsystems|GetEIKSubsystem) (delegate Custom|Session%20Found) (Utilities|Map|MakeMap "" "") "MT_MatchMakingSession" "RE_NoSelection"))

(event Custom|Get%20IP
  ;[1 1 1] Get IP Address
  (Utilities|IsValid (Variables|Default|GetIP%20Finder)
    (:Is%20Valid
      _)
    (:Is%20Not%20Valid
      (bind _returnvalue (Game|ConstructObjectfromClass "/Script/WhatsMyPublicIP.WhatsMyPublicIP"))
      (bind _output_get (Variables|Default|SetIP%20Finder _returnvalue))
      (EventDispatchers|BindEventtoOnIPAddressReceived _output_get (delegate Custom|IP%20Received))))
  (Class|WhatsMyPublicIP|GetMyPublicIP _output_get))

(event Custom|Session%20Found
  (params (bWasSuccess :type Boolean) (SessionResults :type Array%20of%20Session%20Find%20Struct%20Structures))
  ;[1 1 1] Joining EOS Session
  (Class|EIKSubsystem|JoinEosSession (Subsystems|GetEIKSubsystem) (delegate Custom|Join%20Session) "Default_Session" true (.sessionresult (Utilities|Array|Get(acopy) SessionResults))))

(event Custom|Get%20voice%20room%20token
  (params (bWasSuccess :type Boolean) (RoomData :type String))
  ;[1 1 1] Join EOS Voice Room
  (if bWasSuccess
    (Class|EVIKFunctions|JoinEOSRoom (Game|GetPlayerController 0) "BowlingGame" RoomData (delegate Custom|Join%20EOS%20voice%20Room))))

(event EventInit
  (bind _returnvalue (Game|GetPlayerController 0))
  (if (not (Networking|IsDedicatedServer))
    (Development|PrintString "Game Instance" true true "(R=1.000000,G=0.184895,B=0.000000,A=1.000000)" 5.0)
    (CallFunction|GetIP)
    (Class|EIKSubsystem|InitializeEIK (Subsystems|GetEIKSubsystem))
    (Utilities|FlowControl|Delay 1.0)
    (Development|PrintString (Utilities|GetDisplayName _returnvalue) true true "(R=0.000000,G=1.000000,B=0.818574,A=1.000000)" 2e+01)
    (bind _asbp_vrcharacter (Utilities|Casting|CastToBP_VRCharacter (Pawn|GetControlledPawn _returnvalue)))
    (Game|SpawnActorfromClass "/Game/Blueprints/Widgets/LoginWidget/3DLoginWidget.3DLoginWidget_C" (Math|Transform|MakeTransform (Math|Vector|MakeVector (+ (.x (Transformation|GetActorLocation _asbp_vrcharacter)) 3e+02) (.y (Transformation|GetActorLocation _asbp_vrcharacter)) 215.0) "0.000000,-180.000000,0.000000" "0.500000,0.500000,0.500000") "AlwaysSpawn" 0 (Variables|/Game/Blueprints/CharacterClasses/BP_Teleport_Controller.BP_Teleport_Controller_C|GetWidgetInteraction (Variables|/Game/Blueprints/CharacterClasses/BP_VRCharacter.BP_VRCharacter_C|GetTeleportControllerRight _asbp_vrcharacter)) 0)
    (Development|PrintString "Waiting to Join" true true "(R=1.000000,G=0.000000,B=0.007460,A=1.000000)" 5.0)
    (Development|PrintString "Hello" true true "(R=1.000000,G=0.000000,B=0.007460,A=1.000000)" 1e+01)
    (Utilities|FlowControl|Delay 1e+01)
    (Development|ExecuteConsoleCommand "open 127.0.0.1:7777" 0)))